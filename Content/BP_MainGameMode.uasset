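; BP_MainGameMode is the game mode that tracks the current and best score and shows both on screen.
; On BeginPlay it creates the BP_MainWidget HUD and loads the saved best score into it.
; AddScore updates the current score and, when it beats the best, updates the display and immediately saves the new record.
; The best score persists through a BP_SaveData object in the BEST_SCORE save slot.
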(event `self.ReceiveBeginPlay`
  (bind _returnvalue (`|CreateWidget` "/Game/Blueprints/BP_MainWidget.BP_MainWidget_C"))
  (bind _output_get (set `self.MainUI` _returnvalue))
  (`UserWidget.AddToViewport` _output_get 0)
  (`self.LoadData`))

(fn `AddScore`
  (params (AddValue :type Integer))
  (bind _output_get (set `self.CurrScore` (+ AddValue (`self.CurrScore`))))
  (`/Game/Blueprints/BP_MainWidget.Update Curr Score` (`self.MainUI`) _output_get)
  (if (> (`self.CurrScore`) (`self.BestScore`))
    (bind _output_get_2 (set `self.BestScore` (`self.CurrScore`)))
    (`/Game/Blueprints/BP_MainWidget.UpdateBestScore` (`self.MainUI`) _output_get_2)
    (`self.SaveData`)))

(fn `LoadData`
  (bind _returnvalue (`GameplayStatics.LoadGameFromSlot` "BEST_SCORE"))
  (bind _asbp_save_data (cast `/Game/Blueprints/BP_SaveData` _returnvalue))
  (bind _output_get (set `self.BestScore` (`/Game/Blueprints/BP_SaveData.SaveBestScore` _asbp_save_data)))
  (`/Game/Blueprints/BP_MainWidget.UpdateBestScore` (`self.MainUI`) _output_get))

(fn `SaveData`
  (bind _returnvalue (`GameplayStatics.CreateSaveGameObject` "/Game/Blueprints/BP_SaveData.BP_SaveData_C"))
  (set `/Game/Blueprints/BP_SaveData.SaveBestScore` (`self.BestScore`) _returnvalue)
  (`GameplayStatics.SaveGameToSlot` _returnvalue "BEST_SCORE"))

(fn `UserConstructionScript`)
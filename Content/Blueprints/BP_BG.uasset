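; BP_BG is a looping background actor that scrolls downward, judging by its name and movement.
; Every tick it moves along the negative world up vector at a constant speed, scaled by delta time for frame-rate independence.
; When its Z drops below a lower limit, it jumps up by a fixed offset, so the scroll repeats endlessly.
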(event `self.ReceiveTick`
  (params (DeltaSeconds :type "Float (single-precision)"))
  (bind (_returnvalue_x _returnvalue_y _returnvalue_z) (`KismetMathLibrary.BreakVector` (`self.K2_GetActorLocation`)))
  (`self.K2_SetActorLocation` (+ (`self.K2_GetActorLocation`) (* (* (`KismetMathLibrary.GetUpVector` (struct)) -500.0) DeltaSeconds)))
  (if (< _returnvalue_z -5000.0)
    (`self.K2_SetActorLocation` (+ (`self.K2_GetActorLocation`) (0.0 0.0 15000.0)))))

(fn `UserConstructionScript`)
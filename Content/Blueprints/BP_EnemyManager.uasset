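; BP_EnemyManager is a spawner actor that creates BP_Enemy instances at its own transform at random intervals.
; Tick accumulates delta time and spawns an enemy once it reaches the current creation time, then resets the timer.
; SetRandomCreateTime picks the next delay from a short random range, both at BeginPlay and after each spawn.
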(event `self.ReceiveBeginPlay`
  (`self.SetRandomCreateTime`))

(event `self.ReceiveTick`
  (params (DeltaSeconds :type "Float (single-precision)"))
  ;[1 1 1] 시간을 누적시킨다( 시간을 흐르게)
  (set `self.CurrTime` (+ DeltaSeconds (`self.CurrTime`)))
  ;[1 1 1] 일정시간이 지났다면
  (if (>= (`self.CurrTime`) (`self.CreateTime`))
    ;[1 1 1] 나의 위치에 Enemy 를 생성한다.
    (`|SpawnActorFromClass` "/Game/Blueprints/BP_Enemy.BP_Enemy_C" (`self.GetTransform`) "Undefined" "MultiplyWithRoot" null null)
    ;[1 1 1] 현재시간 초기화
    (set `self.CurrTime` 0.0)
    (`self.SetRandomCreateTime`)))

(fn `SetRandomCreateTime`
  ;[1 1 1] 랜덤한 생성시간을 설정하자
  (set `self.CreateTime` (`KismetMathLibrary.RandomFloatInRange` 1.0 3.0)))

(fn `UserConstructionScript`)
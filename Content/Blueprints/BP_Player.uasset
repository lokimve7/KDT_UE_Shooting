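; Player Blueprint for a shooter that moves from axis input and fires bullets from two muzzle points.
; Tick offsets the actor along its up and right vectors by normalized input, Speed and delta time, without sweeping.
; Pressing Fire calls BulletMaKe per muzzle, spawning BP_Bullet and playing a 2D blaster sound.
; A timed-fire remnant still accumulates time, but its branch is empty and its spawn-and-reset nodes are disconnected.
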(event `self.ReceiveTick`
  (params (DeltaSeconds :type "Float (single-precision)"))
  (`self.K2_SetActorLocation` (+ (`self.K2_GetActorLocation`) (* DeltaSeconds (* (`self.Speed`) (`KismetMathLibrary.Normal` (+ (* (`self.GetInputAxisValue`) (`self.GetActorUpVector`)) (* (`self.GetInputAxisValue`) (`self.GetActorRightVector`))))))))
  ;[1 1 1] 시간 누적(시간을 흐르게 한다)
  (bind _output_get (set `self.CurrTime` (+ (`self.CurrTime`) DeltaSeconds)))
  ;[1 1 1] 일정시간이 지나면
  (if (>= _output_get (`self.CreateTime`))
    _))

(event `InputAction|Fire`
  (params (Key :type "Key Structure"))
  ;[1 1 1] 총알 발사
  (:`Pressed`
    (`self.Bullet Ma Ke` (`SceneComponent.K2_GetComponentToWorld` (`self.FirePos01`)))
    (`self.Bullet Ma Ke` (`SceneComponent.K2_GetComponentToWorld` (`self.FirePos02`)))))

(fn `Bullet Ma Ke`
  (params (FirePos :type "Transform Structure"))
  (`|SpawnActorFromClass` "/Game/Blueprints/BP_Bullet.BP_Bullet_C" FirePos "Undefined" "MultiplyWithRoot" null null)
  (`GameplayStatics.PlaySound2D` "/Game/Resources/star-wars-blaster.star-wars-blaster" 1.0 1.0 0.0 null null))

(fn `UserConstructionScript`)
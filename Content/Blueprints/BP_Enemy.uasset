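; BP_Enemy is a shooter enemy that moves in a straight line and explodes on contact.
; On BeginPlay it has a 30% chance to aim at the player's current position, otherwise, or with no player, it heads down its negative up vector.
; Tick moves it along that fixed direction at Speed.
; Overlapping anything except BP_DestroyZone plays an explosion sound and effect, then destroys both actors.
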(event `self.ReceiveBeginPlay`
  (bind _returnvalue (`GameplayStatics.GetActorOfClass` "/Game/Blueprints/BP_Player.BP_Player_C"))
  (bind _output_get (set `self.Player` _returnvalue))
  (`/Engine/EditorBlueprintResources/StandardMacros.IsValid` _output_get
    (:`Is Valid`
      ;[1 1 1] 30%확률로 True, 70% 확률로 False
      (if (< (`KismetMathLibrary.RandomIntegerInRange` 0 9) 3)
        ;[1 1 1] 플레이어를 향하는 방향을 구해자.(타겟(Player).위치 - 나(Enemy).위치)
        (set `self.Direction` (`KismetMathLibrary.Normal` (- (`self.K2_GetActorLocation` (`self.Player`)) (`self.K2_GetActorLocation`))))
        (else
          ;[1 1 1] 방향을 아래로
          (set `self.Direction` (* (`self.GetActorUpVector`) -1.0) :!label _label))))
    (:`Is Not Valid`
      (goto _label))))

(event `self.ReceiveTick`
  (params (DeltaSeconds :type "Float (single-precision)"))
  (`self.K2_SetActorLocation` (+ (`self.K2_GetActorLocation`) (* DeltaSeconds (* (`self.Direction`) (`self.Speed`))))))

(event `self.Collision.OnComponentBeginOverlap`
  (params (OverlappedComponent :type "PrimitiveComponent Object Reference") (OtherActor :type "Actor Object Reference") (OtherComp :type "PrimitiveComponent Object Reference") (OtherBodyIndex :type Integer) (bFromSweep :type Boolean) (SweepResult :type "HitResult Structure (by ref)"))
  (cast `/Game/Blueprints/BP_DestroyZone` OtherActor
    (:`CastFailed`
      ;[1 1 1] 터지는 소리 내자
      (`GameplayStatics.PlaySound2D` "/Game/StarterContent/Audio/Explosion01.Explosion01" 1.0 1.0 0.0 null null)
      ;[1 1 1] 터지는 효과
      (`GameplayStatics.SpawnEmitterAtLocation` "/Game/StarterContent/Particles/P_Explosion.P_Explosion" (`self.K2_GetActorLocation`))
      ;[1 1 1] 부딪힌놈 삭제
      (`self.K2_DestroyActor` OtherActor)
      ;[1 1 1] 나를 삭제
      (`self.K2_DestroyActor`))))

(fn `UserConstructionScript`)
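; BP_Study is a Blueprint scripting practice asset that exercises variables, branching, functions and loops through printed output.
; On BeginPlay it sets and prints Number1, compares it with Number2, prints their total from the Sum function, then prints multiples of three from a for loop.
; A Minus function prints the difference but is never called here, and NewFunction, Tick, overlap and the construction script are empty.
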(event `self.ReceiveBeginPlay`
  ;[1 1 1] Number1 의 값을 출력
  (bind _output_get (set `self.Number1` 200))
  (`KismetSystemLibrary.PrintString` (`KismetStringLibrary.Conv_IntToString` _output_get))
  ;[1 1 1] 조건문 실습
  (if (> (`self.Number1`) (`self.Number2`))
    (`KismetSystemLibrary.PrintString` "Number1 이 큽니다.")
    (else
      (`KismetSystemLibrary.PrintString` "Number2 가 큽니다.")))
  ;[1 1 1] 함수 실습
  (bind _result (`self.Sum` (`self.Number1`) (`self.Number2`)))
  (`KismetSystemLibrary.PrintString` (`KismetStringLibrary.Conv_IntToString` _result))
  ;[1 1 1] 반복문 실습
  (for _index (range 10)
    (`KismetSystemLibrary.PrintString` (`KismetStringLibrary.Conv_IntToString` (* _index 3)) true true (struct :`G` 0.66 :`B` 1.0 :`A` 1.0) 5.0) ; 출력하는 노드
  ))

(event `self.ReceiveTick`
  (params (DeltaSeconds :type "Float (single-precision)")))

(fn `Minus`
  (`KismetSystemLibrary.PrintString` (`KismetStringLibrary.Conv_IntToString` (- (`self.Number1`) (`self.Number2`)))))

(fn `NewFunction`)

(fn `Sum`
  (params (Num1 :type Integer) (Num2 :type Integer))
  (returns (Result :type Integer))
  (return (+ Num1 Num2)))

(fn `UserConstructionScript`)